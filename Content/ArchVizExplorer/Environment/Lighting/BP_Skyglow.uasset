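; BP_Skyglow is an ArchViz Explorer lighting actor that renders a configurable skyglow on a sphere mesh.
; Its construction script creates a dynamic material instance from the sphere's material and pushes the actor's variables into it.
; These set emissive color and intensity, plus opacity shaped by Fresnel, distance-based near/far values and depth fade.
; It has no active runtime logic, as the event graph holds only disabled stub events.
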(event EventBeginPlay)

(event Collision|EventActorBeginOverlap
  (params (OtherActor :type Actor%20Object%20Reference)))

(event EventTick
  (params (DeltaSeconds :type Float%20%28single-precision%29)))

(fn ConstructionScript
  (bind _sphere (Variables|Default|GetSphere))
  (bind _returnvalue (Rendering|Material|CreateDynamicMaterialInstance _sphere 0 (Rendering|Material|GetMaterial _sphere 0) "None" :!class /Script/Engine.PrimitiveComponent))
  (Variables|Default|SetSkyglow_MID _returnvalue)
  ;[1 1 1] Emissive
  (Rendering|Material|SetVectorParameterValue (Variables|Default|GetSkyglow_MID) "Emissive_Color" (Variables|Default|GetEmissive_Color) :!class /Script/Engine.MaterialInstanceDynamic)
  (Rendering|Material|SetScalarParameterValue (Variables|Default|GetSkyglow_MID) "Emissive_Intensity" (Variables|Default|GetEmissive_Intensity) :!class /Script/Engine.MaterialInstanceDynamic)
  ;[1 1 1] Opacity
  (Rendering|Material|SetScalarParameterValue (Variables|Default|GetSkyglow_MID) "Opacity_Fresnel_Power" (Variables|Default|GetOpacity_Fresnel_Power) :!class /Script/Engine.MaterialInstanceDynamic)
  (Rendering|Material|SetScalarParameterValue (Variables|Default|GetSkyglow_MID) "Opacity_Distance_Start" (Variables|Default|GetOpacity_Distance_Start) :!class /Script/Engine.MaterialInstanceDynamic)
  (Rendering|Material|SetScalarParameterValue (Variables|Default|GetSkyglow_MID) "Opacity_Distance_End" (Variables|Default|GetOpacity_Distance_End) :!class /Script/Engine.MaterialInstanceDynamic)
  (Rendering|Material|SetScalarParameterValue (Variables|Default|GetSkyglow_MID) "Opacity_Near" (Variables|Default|GetOpacity_Near) :!class /Script/Engine.MaterialInstanceDynamic)
  (Rendering|Material|SetScalarParameterValue (Variables|Default|GetSkyglow_MID) "Opacity_Far" (Variables|Default|GetOpacity_Far) :!class /Script/Engine.MaterialInstanceDynamic)
  (Rendering|Material|SetScalarParameterValue (Variables|Default|GetSkyglow_MID) "Opacity_DepthFade_Distance" (Variables|Default|GetOpacity_DepthFade_Distance) :!class /Script/Engine.MaterialInstanceDynamic))