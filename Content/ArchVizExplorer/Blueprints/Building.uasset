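; Building actor for an architectural visualization project that toggles its floor components' visibility from a key press.
; On BeginPlay it caches the root's direct child components unless a flag is set.
; The 7 key runs a floor check with a fixed level and prints debug text.
; The check toggles every cached component, using its numeric first-tag comparison against that level only as the propagate-to-children argument.
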(event Custom|checkFloor
  (params (B :type Integer))
  (for _array_element (Variables|Default|GetChildren_0)
    (Rendering|ToggleVisibility _array_element (> (Math|Conversions|ToInteger(Byte) (Utilities|String|ToString(Name) (Utilities|Array|Get(acopy) (Variables|/Script/Engine.ActorComponent|GetComponentTags _array_element)))) B))))

(event EventBeginPlay
  (if (not (Variables|Default|GetNewVar))
    (Variables|Default|SetChildren_0 (Components|GetChildrenComponents (Variables|Default|GetDefaultSceneRoot) false))))

(event Collision|EventActorBeginOverlap
  (params (OtherActor :type Actor%20Object%20Reference)))

(event EventTick
  (params (DeltaSeconds :type Float%20%28single-precision%29)))

(event Input|KeyboardEvents|7
  (params (Key :type Key%20Structure :default "None"))
  (:Pressed
    (CallFunction|CheckFloor 3)
    (Development|PrintString "00000")))

(fn ConstructionScript)